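; BP_Player_Base is the base player character Blueprint, providing a caped body with switchable colors.
; The construction script makes the cape mesh follow the body mesh's pose through a leader pose component.
; Color setters apply indexed materials from BodyMats and CapeMats, and getters look up the current index, though both getters search CapeMats, even for body color.
; It also supplies a fixed camera offset and accessors for GenerateToolType.
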(fn `GetBodyColor`
  (returns (ReturnValue :type Integer))
  (return (`KismetArrayLibrary.Array_Find` (`self.CapeMats`) (`PrimitiveComponent.GetMaterial` (`self.Mesh`) 0))))

(fn `GetCameraOffset`
  (returns (ReturnValue :type "Vector Structure"))
  (return (0.0 25.0 40.0)))

(fn `GetCapeColor`
  (returns (ReturnValue :type Integer))
  (return (`KismetArrayLibrary.Array_Find` (`self.CapeMats`) (`PrimitiveComponent.GetMaterial` (`self.CapeMesh`) 0))))

(fn `GetGenerateToolType`
  (returns (ReturnValue :type "EVoxelGenerateToolType Enum"))
  (return (`self.GenerateToolType`)))

(fn `SetBodyColor`
  (params (InColorIndex :type Integer))
  (`PrimitiveComponent.SetMaterial` (`self.Mesh`) 0 (`|GetArrayItem` (`self.BodyMats`) InColorIndex)))

(fn `SetCapeColor`
  (params (InColorIndex :type Integer))
  (`PrimitiveComponent.SetMaterial` (`self.CapeMesh`) 0 (`|GetArrayItem` (`self.CapeMats`) InColorIndex)))

(fn `SetGenerateToolType`
  (params (InGenerateToolType :type "EVoxelGenerateToolType Enum" :default "None"))
  (set `self.GenerateToolType` InGenerateToolType))

(fn `UserConstructionScript`
  (`SkinnedMeshComponent.SetLeaderPoseComponent` (`self.CapeMesh`) (`self.Mesh`) false false) ; Set cape mesh to match animations of player mesh
)