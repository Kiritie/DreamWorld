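; BP_PlayerCharacter is the player character Blueprint, handling visibility toggling and cape mesh setup.
; SetVisible propagates visibility from the capsule to all child components, then re-hides the big decal and mesh highlight when showing the character.
; The construction script runs the parent's script, then sets the body mesh as the cape's master pose component so the cape follows the player's animations.
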(event `self.SetVisible`
  (params (bVisible :type Boolean))
  (`SceneComponent.SetVisibility` (`self.CapsuleComponent`) bVisible true)
  (if bVisible
    (`SceneComponent.SetVisibility` (`self.BigDecal`) false false)
    (`SceneComponent.SetVisibility` (`self.Mesh highlight`) false false)))

(fn `UserConstructionScript`
  (`parent.UserConstructionScript`)
  (`SkinnedMeshComponent.SetLeaderPoseComponent` (`self.Cape`) (`self.Mesh`) false) ; Set cape mesh to match animations of player mesh
)