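; Rogue player character Blueprint that extends its parent with selectable body and cape colors and a class-specific camera offset.
; Body and cape colors are material-array indices, applied to and read back from the meshes, and the cape follows the body's animation via leader pose.
; A hammer shows only in Creating control mode while visible, and visibility changes always keep the decal and highlight mesh hidden.
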(event `SceneActorInterface.SetActorVisible`
  (params (bInVisible :type Boolean))
  (`parent.SetActorVisible` bInVisible)
  (`SceneComponent.SetVisibility` (`self.BigDecal`) false false)
  (`SceneComponent.SetVisibility` (`self.Mesh highlight`) false false))

(event `self.SetBodyColor`
  (params (InColorIndex :type Integer))
  (`PrimitiveComponent.SetMaterial` (`self.Mesh`) 0 (`|GetArrayItem` (`self.BodyMats`) InColorIndex)))

(event `self.SetCapeColor`
  (params (InColorIndex :type Integer))
  (`PrimitiveComponent.SetMaterial` (`self.Cape`) 0 (`|GetArrayItem` (`self.CapeMats`) InColorIndex)))

(fn `GetBodyColor`
  (returns (ReturnValue :type Integer))
  (return (`KismetArrayLibrary.Array_Find` (`self.BodyMats`) (`PrimitiveComponent.GetMaterial` (`self.Mesh`) 0))))

(fn `GetCameraOffset`
  (returns (ReturnValue :type "Vector Structure"))
  (return (0.0 25.0 45.0)))

(fn `GetCapeColor`
  (returns (ReturnValue :type Integer))
  (return (`KismetArrayLibrary.Array_Find` (`self.CapeMats`) (`PrimitiveComponent.GetMaterial` (`self.Cape`) 0))))

(fn `SetControlMode`
  (params (InControlMode :type "EDWCharacterControlMode Enum" :default "Fighting"))
  (`parent.SetControlMode` InControlMode)
  (`SceneComponent.SetVisibility` (`self.Hammer`) (and (`|EnumEquality` InControlMode "Creating") (`SceneActorInterface.IsVisible`)) false))

(fn `UserConstructionScript`
  (`parent.UserConstructionScript`)
  (`SkinnedMeshComponent.SetLeaderPoseComponent` (`self.Cape`) (`self.Mesh`) false false) ; Set cape mesh to match animations of player mesh
)