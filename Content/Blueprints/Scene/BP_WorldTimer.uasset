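; BP_WorldTimer is the world clock Blueprint, wrapping a DynamicSky object that holds the game's date, time of day and day/night lengths.
; Lifecycle events reset the date on initialize, start time flow in the preparatory phase, and toggle the sky's TimeSpeed on pause and unpause.
; Getters and setters forward to DynamicSky, while sunrise, noon and sunset are fixed fractions of a 2400-unit day rather than values read from the sky.
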(event `self.OnInitialize`
  (`self.ResetDateTime` -1.0))

(event `self.OnPreparatory`
  (set `/UltraDynamicSky/Blueprints/Ultra_Dynamic_Sky.Time Speed` 1.0 (`self.DynamicSky`)))

(event `self.OnRefresh`
  (params (DeltaSeconds :type "Float (single-precision)")))

(event `self.OnPause`
  (set `/UltraDynamicSky/Blueprints/Ultra_Dynamic_Sky.Time Speed` 0.0 (`self.DynamicSky`)))

(event `self.OnUnPause`
  (set `/UltraDynamicSky/Blueprints/Ultra_Dynamic_Sky.Time Speed` 1.0 (`self.DynamicSky`)))

(fn `GetDateTime`
  (returns (ReturnValue :type "DateTime Structure"))
  (bind _current_date_and_time (`/UltraDynamicSky/Blueprints/Ultra_Dynamic_Sky.Get Current Date and Time` (`self.DynamicSky`)))
  (return _current_date_and_time))

(fn `GetDayLength`
  (returns (ReturnValue :type "Float (single-precision)"))
  (return (`/UltraDynamicSky/Blueprints/Ultra_Dynamic_Sky.Day Length` (`self.DynamicSky`))))

(fn `GetNightLength`
  (returns (ReturnValue :type "Float (single-precision)"))
  (return (`/UltraDynamicSky/Blueprints/Ultra_Dynamic_Sky.Night Length` (`self.DynamicSky`))))

(fn `GetNoonTime`
  (returns (ReturnValue :type "Float (single-precision)"))
  (return (* 2400.0 0.5)))

(fn `GetSunriseTime`
  (returns (ReturnValue :type "Float (single-precision)"))
  (return (* 2400.0 0.35)))

(fn `GetSunsetTime`
  (returns (ReturnValue :type "Float (single-precision)"))
  (return (* 2400.0 0.7)))

(fn `GetTimeOfDay`
  (returns (ReturnValue :type "Float (single-precision)"))
  (return (`/UltraDynamicSky/Blueprints/Ultra_Dynamic_Sky.Time of Day` (`self.DynamicSky`))))

(fn `SetDateTime`
  (params (InDataTime :type "DateTime Structure"))
  (`/UltraDynamicSky/Blueprints/Ultra_Dynamic_Sky.Set Date and Time` (`self.DynamicSky`) InDataTime))

(fn `SetDayLength`
  (params (InLength :type "Float (single-precision)"))
  (set `/UltraDynamicSky/Blueprints/Ultra_Dynamic_Sky.Day Length` InLength (`self.DynamicSky`)))

(fn `SetNightLength`
  (params (InLength :type "Float (single-precision)"))
  (set `/UltraDynamicSky/Blueprints/Ultra_Dynamic_Sky.Night Length` InLength (`self.DynamicSky`)))

(fn `SetTimeOfDay`
  (params (InTime :type "Float (single-precision)"))
  (set `/UltraDynamicSky/Blueprints/Ultra_Dynamic_Sky.Time of Day` InTime (`self.DynamicSky`)))