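; Base bow weapon Blueprint that animates the bow's skeletal mesh to follow the owning DWCharacter's combat state.
; Tick checks whether the owner is aiming or performing a normal attack, switching between idle-to-aim and idle animations.
; Two DoOnce gates reset each other, so each animation starts only on a state change.
; Draw play rate scales with an owner attribute during normal attacks and is fixed otherwise.
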(event `self.ReceiveTick`
  (params (DeltaSeconds :type "Float (single-precision)"))
  (bind _skeletalmesh (`self.SkeletalMesh`))
  (bind _asdwcharacter (cast `DWCharacter` (`self.GetOwnerActor`)))
  (bind _returnvalue (`DWCharacter.IsAttacking` _asdwcharacter "NormalAttack"))
  (if (or (`DWCharacter.IsAiming` _asdwcharacter) _returnvalue)
    (`/Engine/EditorBlueprintResources/StandardMacros.DoOnce` false :!label _label
      (:`Completed`
        (`SkeletalMeshComponent.PlayAnimation` _skeletalmesh "/Game/Assets/Misc/ArcherAnimsetPro/Animations/Bow/Bow_Idle_2_Aim_Bow.Bow_Idle_2_Aim_Bow" false)
        (`SkeletalMeshComponent.SetPlayRate` _skeletalmesh (select `bool` _returnvalue :`false` 2.5 :`true` (* (`AttributeSetBase.GetAttributeValue` (`AbilityCharacterBase.AttributeSet` _asdwcharacter) (struct :`AttributeName` "AttackSpeed" :`Attribute` "/Script/DreamWorld.DWCharacterAttributeSet:AttackSpeed" :`AttributeOwner` "/Script/CoreUObject.Class'/Script/DreamWorld.DWCharacterAttributeSet'")) 2.0) :!type "Float (single-precision)"))
        (goto _label_2 :!via `Reset`)))
    (else
      (`/Engine/EditorBlueprintResources/StandardMacros.DoOnce` false :!label _label_2
        (:`Completed`
          (`SkeletalMeshComponent.PlayAnimation` _skeletalmesh "/Game/Assets/Misc/ArcherAnimsetPro/Animations/Bow/Bow_Idle_01_Bow.Bow_Idle_01_Bow" false)
          (`SkeletalMeshComponent.SetPlayRate` _skeletalmesh 1.0)
          (goto _label :!via `Reset`))))))

(fn `UserConstructionScript`)