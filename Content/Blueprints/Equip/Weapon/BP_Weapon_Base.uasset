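; Base weapon Blueprint that handles the gameplay and feedback response when the weapon hits a target.
; OnHitTarget sends an Event.Hit.Attack gameplay event to the owning character, with that character as instigator and the hit actor as target.
; It then plays a sound and particle effect at the mesh's HitPoint socket, loaded from the item's weapon data asset.
; Hit or miss variants are chosen by whether the target implements AbilityVitalityInterface.
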(event `self.OnHitTarget`
  (params (OverlappedComponent :type "PrimitiveComponent Object Reference") (OtherActor :type "Actor Object Reference") (OtherComp :type "PrimitiveComponent Object Reference") (OtherBodyIndex :type Integer) (bFromSweep :type Boolean) (SweepResult :type "HitResult Structure (by ref)"))
  (bind _returnvalue (`self.GetOwnerCharacter`))
  (bind _returnvalue_2 (`KismetSystemLibrary.DoesImplementInterface` OtherActor "/Script/WHFramework.AbilityVitalityInterface"))
  (bind _item_id (break `AbilityItem` (`self.Item`)))
  (bind _returnvalue_3 (`AssetModuleBPLibrary.K2_LoadPrimaryAsset` _item_id "/Script/DreamWorld.DWEquipWeaponData"))
  (bind _returnvalue_4 (`SceneComponent.GetSocketLocation` (`self.MeshComponent`) "HitPoint"))
  (`AbilitySystemBlueprintLibrary.SendGameplayEventToActor` _returnvalue (struct :`TagName` "Event.Hit.Attack") (make `GameplayEventData` (struct) _returnvalue OtherActor))
  (`GameplayStatics.PlaySoundAtLocation` (select `bool` _returnvalue_2 :`false` (`DWEquipWeaponData.AttackMissSound` _returnvalue_3) :`true` (`DWEquipWeaponData.AttackHitSound` _returnvalue_3)) _returnvalue_4 (struct) 1.0 1.0 0.0 null null null null)
  (`GameplayStatics.SpawnEmitterAtLocation` (select `bool` _returnvalue_2 :`false` (`DWEquipWeaponData.AttackMissEffect` _returnvalue_3) :`true` (`DWEquipWeaponData.AttackHitEffect` _returnvalue_3)) _returnvalue_4))

(fn `UserConstructionScript`)