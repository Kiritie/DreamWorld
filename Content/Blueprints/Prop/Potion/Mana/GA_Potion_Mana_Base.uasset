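; Base Gameplay Ability for mana potions, with its activation logic left to parent or child classes.
; The activation check casts the owner actor to DWCharacter and allows use only when one AttributeSet value is below another, presumably current mana against maximum, though the attributes are not shown.
; The activate and end events are disabled placeholder nodes.
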(fn `K2_CanActivateAbility`
  (params (ActorInfo :type "GameplayAbilityActorInfo Structure") (Handle :type "GameplayAbilitySpecHandle Structure"))
  (returns (RelevantTags :type "GameplayTagContainer Structure") (ReturnValue :type Boolean))
  (bind _asdwcharacter (cast `DWCharacter` (`.OwnerActor` (break `GameplayAbilityActorInfo` ActorInfo))))
  (bind _attributeset (`AbilityCharacterBase.AttributeSet` _asdwcharacter))
  (return (struct) (< (`AttributeSetBase.GetAttributeValue` _attributeset (struct :`AttributeName` "Mana" :`Attribute` "/Script/DreamWorld.DWCharacterAttributeSet:Mana" :`AttributeOwner` "/Script/CoreUObject.Class'/Script/DreamWorld.DWCharacterAttributeSet'")) (`AttributeSetBase.GetAttributeValue` _attributeset (struct :`AttributeName` "MaxMana" :`Attribute` "/Script/DreamWorld.DWCharacterAttributeSet:MaxMana" :`AttributeOwner` "/Script/CoreUObject.Class'/Script/DreamWorld.DWCharacterAttributeSet'")))))