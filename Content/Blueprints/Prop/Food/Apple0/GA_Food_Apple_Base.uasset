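; GA_Food_Apple_Base is the base gameplay ability for the apple food prop.
; It overrides only the activation check, which casts the owning actor to DWCharacter and passes when one value from its AttributeSet is below another.
; Activation and end events are disabled stubs, so the Blueprint adds no effect logic of its own.
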(fn `K2_CanActivateAbility`
  (params (ActorInfo :type "GameplayAbilityActorInfo Structure") (Handle :type "GameplayAbilitySpecHandle Structure"))
  (returns (RelevantTags :type "GameplayTagContainer Structure") (ReturnValue :type Boolean))
  (bind _asdwcharacter (cast `DWCharacter` (`.OwnerActor` (break `GameplayAbilityActorInfo` ActorInfo))))
  (bind _attributeset (`AbilityCharacterBase.AttributeSet` _asdwcharacter))
  (return (struct) (< (`AttributeSetBase.GetAttributeValue` _attributeset (struct :`AttributeName` "Health" :`Attribute` "/Script/WHFramework.VitalityAttributeSetBase:Health" :`AttributeOwner` "/Script/CoreUObject.Class'/Script/WHFramework.VitalityAttributeSetBase'")) (`AttributeSetBase.GetAttributeValue` _attributeset (struct :`AttributeName` "MaxHealth" :`Attribute` "/Script/WHFramework.VitalityAttributeSetBase:MaxHealth" :`AttributeOwner` "/Script/CoreUObject.Class'/Script/WHFramework.VitalityAttributeSetBase'")))))